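; Game mode Blueprint for Toon Tanks that handles the on-screen UI at match start and end.
; StartGame adds the start widget to the viewport.
; GameOver shows a win or lose message based on WonGame, then removes that text after a short delay and adds the restart widget.
; After a second delay it opens the Main level automatically, with no player input.
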(event EventBeginPlay)

(event EventTick
  (params (DeltaSeconds :type Float%20%28single-precision%29)))

(event EventStartGame
  (bind _returnvalue (UserInterface|CreateWidget "/Game/Blueprints/Widgets/WBP_StartGameWidget.WBP_StartGameWidget_C"))
  (UserInterface|Viewport|AddtoViewport _returnvalue 0))

(event EventGameOver
  (params (bWonGame :type Boolean))
  (bind _returnvalue (UserInterface|CreateWidget "/Game/Blueprints/Widgets/WBP_EndGameWidget.WBP_EndGameWidget_C"))
  (UserInterface|Viewport|AddtoViewport _returnvalue 0)
  (Rendering|Components|TextRender|SetText (Variables|/Game/Blueprints/Widgets/WBP_EndGameWidget.WBP_EndGameWidget_C|GetDisplayText _returnvalue) (select bWonGame "You won!" "You lose!"))
  (Utilities|FlowControl|Delay 2.0)
  (Widget|RemovefromParent (Variables|/Game/Blueprints/Widgets/WBP_EndGameWidget.WBP_EndGameWidget_C|GetDisplayText _returnvalue))
  (bind _returnvalue_2 (UserInterface|CreateWidget "/Game/Blueprints/Widgets/WBP_RestartLevelWidget.WBP_RestartLevelWidget_C"))
  (UserInterface|Viewport|AddtoViewport _returnvalue_2 0)
  (Utilities|FlowControl|Delay 3.0)
  (Game|OpenLevel(byName) "Main"))

(fn ConstructionScript)